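; Actor component that plays footstep, jump and landing sounds for the player character, varying steps and landings by ground surface.
; GetSurface traces 500 units down from player character 0 on Visibility and returns the hit's physical material surface type and impact point.
; PlayFootstep and PlayLand use these to pick and place Snow, Grass, Concrete or Metal sounds, defaulting to Concrete.
; PlayJump plays one sound at a supplied location.
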(fn PlayFootstep
  (bind _concrete_run_sound (Variables|Default|GetConcrete_Run_Sound))
  ;[1 1 1] Play the sound based on returned surface and location
  (bind (_surface _impactpoint) (CallFunction|GetSurface))
  (Audio|SpawnSoundatLocation (Utilities|Select :Index _surface :SurfaceType_Default _concrete_run_sound :SurfaceType1 (Variables|Default|GetSnow_Run_Sound) :SurfaceType2 (Variables|Default|GetGrass_Run_Sound) :SurfaceType3 _concrete_run_sound :SurfaceType4 (Variables|Default|GetMetal_Run_Sound)) _impactpoint "0, 0, 0" 1.0 1.0 0.0 0 0)
  ;[1 1 1] Debug - print surface type
  (Development|PrintString (Utilities|String|EnumtoString _surface)))

(fn GetSurface
  (bind _returnvalue (Game|GetPlayerCharacter 0))
  (bind _returnvalue_2 (Transformation|GetActorLocation _returnvalue))
  (bind (_x _y _z) (Math|Vector|BreakVector _returnvalue_2))
  (bind (_outhit _returnvalue_3) (Collision|LineTraceByChannel _returnvalue_2 (Math|Vector|MakeVector _x _y (- _z 5e+02)) "TraceTypeQuery1" false 0 "None"))
  (if _returnvalue_3
    (return (Variables|/Script/PhysicsCore.PhysicalMaterial|GetSurfaceType (.PhysMat (Collision|BreakHitResult _outhit))) (.ImpactPoint (Collision|BreakHitResult _outhit)))
    (else
      (Development|PrintString "INVALID LINE TRACE RESULT" true true "(R=1.000000,G=0.000000,B=0.032248,A=1.000000)" 5.0))))

(fn PlayJump
  (params (Location :type Vector))
  ;[1 1 1] Single type of jump sound
  (Audio|SpawnSoundatLocation (Variables|Default|GetJump_Sound) Location "0, 0, 0" 1.0 1.0 0.0 0 0))

(fn PlayLand
  (bind _concrete_land_sound (Variables|Default|GetConcrete_Land_Sound))
  ;[1 1 1] Play 'land' sound - get surface and location
  (bind (_surface _impactpoint) (CallFunction|GetSurface))
  (Audio|SpawnSoundatLocation (Utilities|Select :Index _surface :SurfaceType_Default _concrete_land_sound :SurfaceType1 (Variables|Default|GetSnow_Land_Sound) :SurfaceType2 (Variables|Default|GetGrass_Land_Sound) :SurfaceType3 _concrete_land_sound :SurfaceType4 (Variables|Default|GetMetal_Land_Sound)) _impactpoint "0, 0, 0" 1.0 1.0 0.0 0 0))