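; Ambient music manager that plays a random song from its Songs list through a Music audio component, starting on BeginPlay when AutoPlay is set.
; NewSong fades in a random pick if nothing is playing.
; If music is already playing, it fades it out and loops on IsPlaying with debug prints, with no delay in the loop and no new song started afterwards.
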(event EventBeginPlay
  (if (Variables|Default|GetautoPlay?)
    (CallFunction|NewSong)))

(fn ConstructionScript)

(fn NewSong
  (bind _music (Variables|Default|GetMusic))
  (if (Audio|Components|Audio|IsPlaying (Variables|Default|GetMusic))
    (Audio|Components|Audio|FadeOut _music 5.0 0.0 "Linear" :!class /Script/Engine.AudioComponent)
    (while (Audio|Components|Audio|IsPlaying (Variables|Default|GetMusic))
      (Development|PrintString "fading out"))
    (Development|PrintString "Done fading")
    (else
      (Audio|Components|Audio|SetSound _music (.OutItem (Utilities|Array|Random (Variables|Default|Getsongs))))
      (Audio|Components|Audio|FadeIn _music 1.0 1.0 0.0 "Linear" :!class /Script/Engine.AudioComponent))))