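; Trigger actor that switches the environment ambience when the third-person player character enters or leaves its overlap area.
; On BeginPlay it finds and caches the level's Ambience_Manager_BP, printing a red error with its own name if none exists.
; Entering passes its NewEnvironment to the manager's NewAmbience, and leaving passes the manager's DefaultEnvironment, filtered by an exact class match on BP_ThirdPersonCharacter.
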(event Collision|EventActorBeginOverlap
  (params (OtherActor :type Actor%20Object%20Reference))
  (if (== (Utilities|GetClass OtherActor) "/Game/ThirdPerson/Blueprints/BP_ThirdPersonCharacter.BP_ThirdPersonCharacter_C")
    (Default|NewAmbience (Variables|Default|GetambienceManager) (Variables|Default|GetnewEnvironment))))

(event Collision|EventActorEndOverlap
  (params (OtherActor :type Actor%20Object%20Reference))
  (bind _ambiencemanager (Variables|Default|GetambienceManager))
  (if (== (Utilities|GetClass OtherActor) "/Game/ThirdPerson/Blueprints/BP_ThirdPersonCharacter.BP_ThirdPersonCharacter_C")
    (Default|NewAmbience _ambiencemanager (Variables|/Game/Ben_Lusted/Ambience/Ambience_Manager_BP.Ambience_Manager_BP_C|GetdefaultEnvironment _ambiencemanager))))

(event EventBeginPlay
  (bind _returnvalue (Actor|GetActorOfClass "/Game/Ben_Lusted/Ambience/Ambience_Manager_BP.Ambience_Manager_BP_C"))
  (if (Utilities|IsValid _returnvalue)
    (Variables|Default|SetambienceManager _returnvalue)
    (else
      (Development|PrintString (Utilities|String|Append "CANNOT FIND AMBIENCE MANAGER" (Utilities|GetDisplayName self)) true true "(R=1.000000,G=0.000000,B=0.042729,A=1.000000)" 5.0))))

(fn ConstructionScript)