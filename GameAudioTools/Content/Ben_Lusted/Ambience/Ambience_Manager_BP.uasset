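; Ambience manager Blueprint that plays looping background ambience for the current environment: Flatlands, House or Cave.
; On BeginPlay it starts the default environment's ambience when AutoPlay is enabled.
; NewAmbience stores the environment, selects its sound, then alternates between two audio components, crossfading from Ambience1 to Ambience2 or fading Ambience1 in if idle.
; House has no sound assigned, and Ambience2 is never faded out.
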(event EventBeginPlay
  (if (Variables|Default|GetautoPlay)
    (CallFunction|NewAmbience (Variables|Default|GetdefaultEnvironment))))

(fn ConstructionScript)

(fn NewAmbience
  (params (environment :type EEnvironment_Area%20Enum :default "NewEnumerator0"))
  (bind _output_get (Variables|Default|SetcurrentEnvironment environment))
  (Variables|Default|SetnewSound (Utilities|Select :Index _output_get :NewEnumerator0 "/Game/_Example/Waves/Ambience/Flatlands_Amb_LP.Flatlands_Amb_LP" :NewEnumerator1 0 :NewEnumerator2 "/Game/_Example/Waves/Ambience/Caves_Amb_LP.Caves_Amb_LP"))
  (if (Audio|Components|Audio|IsPlaying (Variables|Default|GetAmbience_1))
    ;[1 1 1] Setup and fade in ambience 2
    (Audio|Components|Audio|SetSound (Variables|Default|GetAmbience_2) (Variables|Default|GetnewSound))
    (Audio|Components|Audio|FadeOut (Variables|Default|GetAmbience_1) 1.0 0.0 "Linear" :!class /Script/Engine.AudioComponent)
    (Audio|Components|Audio|FadeIn (Variables|Default|GetAmbience_2) 1.0 1.0 0.0 "Linear" :!class /Script/Engine.AudioComponent)
    (else
      ;[1 1 1] Setup and fade in ambience 1
      (Audio|Components|Audio|SetSound (Variables|Default|GetAmbience_1) (Variables|Default|GetnewSound))
      (Audio|Components|Audio|FadeIn (Variables|Default|GetAmbience_1) 1.0 1.0 0.0 "Linear" :!class /Script/Engine.AudioComponent))))